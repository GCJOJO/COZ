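; BP_GoToQuest is a quest updater that completes a "go to location" quest when the player reaches it.
; Every tick it checks whether the quest matching its QuestID has a specific completion state, setting Activated and the Sphere marker's visibility to match.
; When the Player overlaps its Box while Activated, it clears the flag and completes that quest through the Quests object.
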(event OnComponentBeginOverlap(Box)
  (params (OverlappedComponent :type Primitive%20Component%20Object%20Reference) (OtherActor :type Actor%20Object%20Reference) (OtherComp :type Primitive%20Component%20Object%20Reference) (OtherBodyIndex :type Integer) (bFromSweep :type Boolean) (SweepResult :type Hit%20Result%20Structure%20%28by%20ref%29))
  (Utilities|Casting|CastToPlayer OtherActor)
  (if (Variables|Default|GetActivated)
    (Variables|Default|SetActivated false)
    (Default|CompleteQuest (Variables|Default|GetQuests) (Variables|Default|GetQuestID))))

(event EventBeginPlay
  (|CallParentFunction))

(event Collision|EventActorBeginOverlap
  (params (OtherActor :type Actor%20Object%20Reference))
  (|CallParentFunction OtherActor) ; This node is disabled and will not be called.\nDrag off pins to build functionality.
)

(event EventTick
  (params (DeltaSeconds :type Float%20%28single-precision%29))
  (|CallParentFunction DeltaSeconds)
  (bind _return (Default|IsQuestCompletionEqualto (Variables|Default|GetQuests) (Variables|Default|GetQuestID) "NewEnumerator2"))
  (if _return
    (Variables|Default|SetActivated true)
    (else
      (Variables|Default|SetActivated false)))
  (Rendering|SetVisibility (Variables|Default|GetSphere) (Variables|Default|GetActivated) false))

(fn ConstructionScript
  (|CallParentFunction))
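; Shooting target actor for a tutorial that reacts once to a first-person projectile hit by rotating its mesh.
; BeginPlay snaps the mesh roll to -90 after a delay, and the GetUP event rotates it through the RotateUP timeline.
; While Enabled, a projectile hit on the capsule plays the Rotate timeline, then destroys the capsule and disables the target.
; Timelines drive only roll, and an unconnected debug rotation chain remains.
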(event OnComponentHit(Capsule)
  (params (HitComponent :type Primitive%20Component%20Object%20Reference) (OtherActor :type Actor%20Object%20Reference) (OtherComp :type Primitive%20Component%20Object%20Reference) (NormalImpulse :type Vector :default "0, 0, 0") (Hit :type Hit%20Result%20Structure%20%28by%20ref%29))
  (bind _targetmesh (Variables|Default|GetTargetMesh))
  (bind _returnvalue (Transformation|GetWorldRotation _targetmesh))
  (if (Variables|Default|GetEnabled)
    (Utilities|Casting|CastToFirstPersonProjectile OtherActor)
    (Development|PrintString "Hit !")
    (Utilities|FlowControl|Sequence
      (:then_0
        (bind _x_axis (Timeline|Rotate Play)
          (:Update
            (Transformation|SetWorldRotation _targetmesh (Math|Rotator|MakeRotator _x_axis (.pitch _returnvalue) (.yaw _returnvalue)) false false))))
      (:then_1
        (Components|DestroyComponent (Variables|Default|GetCapsule))
        (Variables|Default|SetEnabled false)))))

(event Custom|GetUP
  (bind _targetmesh (Variables|Default|GetTargetMesh))
  (bind _returnvalue (Transformation|GetWorldRotation _targetmesh))
  (bind _x_axis (Timeline|Rotate%20UP Play)
    (:Update
      (Transformation|SetWorldRotation _targetmesh (Math|Rotator|MakeRotator _x_axis (.pitch _returnvalue) (.yaw _returnvalue)) false false))))

(event EventBeginPlay
  (bind _targetmesh (Variables|Default|GetTargetMesh))
  (bind _returnvalue (Transformation|GetWorldRotation _targetmesh))
  (Utilities|FlowControl|Delay 1e+01)
  (Transformation|SetWorldRotation _targetmesh (Math|Rotator|MakeRotator -9e+01 (.pitch _returnvalue) (.yaw _returnvalue)) false false))

(event Collision|EventActorBeginOverlap
  (params (OtherActor :type Actor%20Object%20Reference)))

(event EventTick
  (params (DeltaSeconds :type Float%20%28single-precision%29)))

(fn ConstructionScript)